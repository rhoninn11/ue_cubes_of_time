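; BP_CubesOfTime draws a trail of small colored cubes that visualizes position history from a linked spatial memory object.
; On BeginPlay it spawns collision-free cube components, each tinted by a dynamic material from a color curve, and initializes position and speed arrays.
; follow_me sets the memory source; each Tick samples its history and teleports the cubes to those points.
; Per-cube frame-to-frame deltas are stored as speeds but not used here.
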(event `self.ReceiveBeginPlay`
  (bind _cube_num (`self.cube_num`))
  ;[1 1 1] startujemy_kuleczki
  (`|ExecutionSequence`
    (:`then_0`
      (`self.Populate Cubes` _cube_num))
    (:`then_1`
      (`self.init_points` _cube_num))))

(event `follow_me`
  (params (higher_level_of_spatioal_memory :type "/cubes_of_time/BP_space_time_memory Object Reference"))
  ;[1 1 1] zwiazanie
  (set `self.higher_level_of_spatioal_memory` higher_level_of_spatioal_memory))

(event `self.ReceiveTick`
  (params (DeltaSeconds :type "Float (single-precision)"))
  (`|ExecutionSequence`
    (:`then_0`
      ;[1 1 1] zwiazanie
      (bind _sampled_pos (`/cubes_of_time/BP_space_time_memory.sample_history` (`self.higher_level_of_spatioal_memory`) (`self.cube_num`) 20))
      (set `self.cube_pos_then` (`self.cube_pos_now`))
      (set `self.cube_pos_now` _sampled_pos))
    (:`then_1`
      ;[1 1 1] to_jeszcze_niepewne
      (`self.calc_speed`))
    (:`then_2`
      (`self.signal_cubes`))))

(fn `calc_speed`
  (for _index (range (`self.cube_num`))
    (`KismetArrayLibrary.Array_Set` (`self.cube_speed`) _index (- (`|GetArrayItem` (`self.cube_pos_now`) _index) (`|GetArrayItem` (`self.cube_pos_then`) _index)))))

(fn `init_points`
  (params (point_num :type Integer))
  (locals (initail_pos :type "Vector Structure") (initial_speed :type "Vector Structure"))
  (bind _cube_pos_now (`self.cube_pos_now`))
  (bind _cube_speed (`self.cube_speed`))
  (bind _cube_pos_then (`self.cube_pos_then`))
  (`|ExecutionSequence`
    (:`then_0`
      (`KismetArrayLibrary.Array_Clear` _cube_pos_now)
      (for _ (range point_num)
        (`KismetArrayLibrary.Array_Add` _cube_pos_now (`local.initail_pos`))))
    (:`then_1`
      (`KismetArrayLibrary.Array_Clear` _cube_speed)
      (for _ (range point_num)
        (`KismetArrayLibrary.Array_Add` _cube_speed (`local.initial_speed`))))
    (:`then_2`
      (`KismetArrayLibrary.Array_Clear` _cube_pos_then)
      (for _ (range point_num)
        (`KismetArrayLibrary.Array_Add` _cube_pos_then (`local.initail_pos`))))))

(fn `Populate Cubes`
  (params (n :type Integer))
  (locals (progression :type "Float (double-precision)"))
  (bind _past_cubes (`self.past_cubes`))
  (`KismetArrayLibrary.Array_Clear` _past_cubes)
  (for _index (range n)
    (bind _output_get (set `local.progression` (/ (`KismetMathLibrary.Conv_IntToDouble` _index) (- (`self.max_cube_num`) 1))))
    (`self.spawn_nth_cube` _past_cubes _output_get)))

(fn `signal_cubes`
  (`|ExecutionSequence`
    (:`then_0`
      (for (_array_element _array_index) (`self.past_cubes`)
        (`SceneComponent.K2_SetWorldLocation` _array_element (`|GetArrayItem` (`self.cube_pos_now`) _array_index) false true)))
    (:`then_1`
      (for _ (`self.past_cubes`)
        _))))

(fn `spawn_nth_cube`
  (params (InputPin :type "Array of StaticMeshComponent Object Reference") (progress :type "Float (double-precision)"))
  (bind _returnvalue (`AddComponent|NODE_AddStaticMeshComponent-0` :`RelativeTransform` (`KismetMathLibrary.MakeTransform` (0.0 0.0 0.0) (struct) (`KismetMathLibrary.Conv_DoubleToVector` 0.06))))
  (`PrimitiveComponent.SetCollisionEnabled` _returnvalue "NoCollision")
  (`KismetArrayLibrary.Array_Add` InputPin _returnvalue)
  (bind _returnvalue_2 (`PrimitiveComponent.CreateDynamicMaterialInstance` _returnvalue 0 "/cubes_of_time/colored_trace.colored_trace" "None"))
  (`MaterialInstanceDynamic.SetVectorParameterValue` _returnvalue_2 "color" (`CurveLinearColor.GetLinearColorValue` (`self.color_ref`) progress)))

(fn `UserConstructionScript`)