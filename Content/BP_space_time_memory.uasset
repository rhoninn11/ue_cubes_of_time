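; Space-time memory component that records its recent world positions and per-tick displacements, and registers with a BP_CubesOfTime to be followed.
; On readiness it fills fixed-length histories with the starting position and initial speed.
; While tracing, each tick shifts in the current position, using a second, one-step-behind buffer to derive velocity as position deltas.
; An index-capped getter exposes past locations; debug prints remain.
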(event `self.ReceiveBeginPlay`
  (`self.check_readyness`))

(event `check_readyness`
  (bind _external_cubes (`self.external_cubes`))
  (`|ExecutionSequence`
    (:`then_0`
      ;[0 0 0] bond with cubes
      (`/Engine/EditorBlueprintResources/StandardMacros.IsValid` _external_cubes
        (:`Is Valid`
          (bind _asbp_cubes_of_time (cast `/cubes_of_time/BP_CubesOfTime` _external_cubes))
          (`/cubes_of_time/BP_CubesOfTime.follow_me` _asbp_cubes_of_time self)
          (set `self.has_valid_ref` true))))
    (:`then_1`
      ;[0 0 0] ready_for_sim
      (if (`self.has_valid_ref`)
        (`self.obserwator_gotowy` self)))))

(event `self.ReceiveTick`
  (params (DeltaSeconds :type "Float (single-precision)"))
  ;[0 0 0] simulate
  (if (and (`self.to_trace`) (`self.has_valid_ref`))
    (`self.obserwator_leci` self)
    (`KismetSystemLibrary.PrintString` "Hello")))

(event `obserwator_gotowy`
  (params (for_component :type "SceneComponent Object Reference"))
  ;[1 1 1] a jak by w grafach tez zbierac eventy, to chyba strona a
  (`self.a_ready` for_component))

(event `po`
  ;[1 1 1] to teraz jeszcze dla strony b
)

(event `obserwator_leci`
  (params (for_component :type "SceneComponent Object Reference"))
  ;[1 1 1] a jak by w grafach tez zbierac eventy, to chyba strona a
  (`self.a_simulate` for_component))

(fn `a_ready`
  (params (for_component :type "SceneComponent Object Reference"))
  (locals (init_pos :type "Vector Structure" :default (0.0 0.0 0.0)) (init_vel :type "Vector Structure"))
  (`self.init_whole_history` (`KismetMathLibrary.TransformLocation` (`self.K2_GetComponentToWorld` for_component))))

(fn `a_simulate`
  (params (for_component :type "SceneComponent Object Reference"))
  (locals (ops_comp :type "SceneComponent Object Reference"))
  (set `local.ops_comp` for_component)
  (`|ExecutionSequence`
    (:`then_0`
      ;[0 0 0] sample space position
      (`self.V Push And Shift` (`self.history_of_pos`) (`KismetMathLibrary.TransformLocation` (`self.K2_GetComponentToWorld` (`local.ops_comp`)))))
    (:`then_1`
      (`self.calc_history_delta` (`self.history_of_pos`) (`self.history_of_posi`) (`self.history_of_vel`)))
    (:`then_2`
      (`self.V Push And Shift` (`self.history_of_posi`) (`KismetMathLibrary.TransformLocation` (`self.K2_GetComponentToWorld` (`local.ops_comp`)))))))

(fn `b_get_location_in_time`
  (params (location_idx :type Integer))
  (returns (pash_hand_location :type "Vector Structure"))
  (bind _returnvalue (`KismetArrayLibrary.Array_Length` (`self.history_of_pos`)))
  (return (`|GetArrayItem` (`self.history_of_pos`) (`KismetMathLibrary.SelectInt` location_idx (- _returnvalue 1) (< location_idx _returnvalue)))))

(fn `calc_history_delta`
  (params (fresh_history :type "Array of Vector Structure") (old_history :type "Array of Vector Structure") (vel_history :type "Array of Vector Structure"))
  (for _index (range (`self._history_len`))
    (`KismetArrayLibrary.Array_Set` vel_history _index (- (`|GetArrayItem` fresh_history _index) (`|GetArrayItem` old_history _index)))))

(fn `init_history`
  (params (len :type Integer) (history_of :type "Array of Vector Structure (by ref)") (pos :type "Vector Structure (by ref)"))
  (for _index (range len)
    (`KismetArrayLibrary.Array_Set` history_of _index pos true))
  (`KismetSystemLibrary.LogString` "+++ inicjalicjalizacja"))

(fn `init_whole_history`
  (params (InputPin :type "Vector Structure"))
  (locals (initial_speed :type "Vector Structure"))
  (`|ExecutionSequence`
    (:`then_0`
      (`self.init_history` (`self._history_len`) (`self.history_of_pos`) InputPin))
    (:`then_1`
      (`self.init_history` (`self._history_len`) (`self.history_of_posi`) InputPin))
    (:`then_2`
      (`self.init_history` (`self._history_len`) (`self.history_of_vel`) (`local.initial_speed`)))))

(fn `V Push And Shift`
  (params (va :type "Array of Vector Structure") (new :type "Vector Structure (by ref)"))
  (for (_array_element _array_index) va
    (if (> _array_index 0)
      (`KismetArrayLibrary.Array_Set` va (- _array_index 1) _array_element)))
  (`KismetArrayLibrary.Array_Set` va _array_index new))

(fn `v_array_log`
  (params (Array :type "Array of Vector Structure"))
  (locals (message :type String))
  (for (_array_element _array_index) Array
    (set `local.message` (`KismetStringLibrary.Concat_StrStr` (`local.message`) (`KismetStringLibrary.Concat_StrStr` (`KismetStringLibrary.Conv_IntToString` _array_index) ": " (`KismetStringLibrary.Conv_VectorToString` _array_element)) " | ")))
  (`KismetSystemLibrary.LogString` (`local.message`)))